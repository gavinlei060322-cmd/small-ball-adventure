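; BP_Spotlight_follow is a spotlight prop that turns to follow the player while they are inside its overlap area.
; Actor begin and end overlap events, filtered by an Isplayer check, toggle the IsPlayerOverlapping flag.
; While the flag is set, Tick smoothly interpolates the SpotLight's world rotation toward a look-at rotation aimed at player pawn 0.
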(event Collision|EventActorBeginOverlap
  (params (OtherActor :type Actor%20Object%20Reference))
  (Utilities|Isplayer OtherActor
    (:true
      (Variables|Default|SetIsPlayerOverlapping true))))

(event EventTick
  (params (DeltaSeconds :type Float%20%28single-precision%29))
  (if (Variables|Default|GetIsPlayerOverlapping)
    (Transformation|SetWorldRotation (Variables|Default|GetSpotLight) (Math|Interpolation|RInterpTo (Transformation|GetWorldRotation (Variables|Default|GetSpotLight)) (Math|Rotator|FindLookatRotation (Transformation|GetWorldLocation (Variables|Default|GetSpotLight)) (Transformation|GetActorLocation (Game|Player|GetPlayerPawn 0))) DeltaSeconds 5.0) false false)))

(event Collision|EventActorEndOverlap
  (params (OtherActor :type Actor%20Object%20Reference))
  (Utilities|Isplayer OtherActor
    (:true
      (Variables|Default|SetIsPlayerOverlapping false))))

(fn ConstructionScript)