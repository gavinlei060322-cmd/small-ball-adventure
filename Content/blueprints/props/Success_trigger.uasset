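; Level exit trigger that lets the player finish a level once every crystal is collected.
; BeginPlay stores the BP_cristal count in the game instance, and player overlap compares it with the collected count.
; If complete, the last level sets IsWin; others save level time, darken the camera, open the next LevelNameList entry and reset the collected count.
; Otherwise, the BP_UI widget plays a flicker animation.
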(event Collision|EventActorBeginOverlap
  (params (OtherActor :type Actor%20Object%20Reference))
  (bind _returnvalue (Math|Float|MakeLiteralFloat 1.0))
  (Utilities|Isplayer OtherActor
    (:true
      (bind _asbp_game_instance (Utilities|ConvertGameInstance))
      (if (== (Variables|/Game/blueprints/props/BP_GameInstance.BP_GameInstance_C|GetAllCristalNumber _asbp_game_instance) (Variables|/Game/blueprints/props/BP_GameInstance.BP_GameInstance_C|GetCollected_Cristal_Number _asbp_game_instance))
        (bind _result (CallFunction|IsLastLevel))
        (if _result
          (bind _asbp_game_instance_2 (Utilities|ConvertGameInstance))
          (Variables|/Game/blueprints/props/BP_GameInstance.BP_GameInstance_C|SetIsWin _asbp_game_instance_2 true)
          (else
            (bind _level_name (CallFunction|GetCurrentLevelIndex))
            (bind _result_2 (Math|Integer|IncrementInt _level_name)
              (:%20%20
                (CallFunction|SaveLevelTime)
                (Utilities|MakeCameraDark :Duration _returnvalue)
                (Utilities|FlowControl|Delay _returnvalue)
                (Game|OpenLevel(byName) (Utilities|Array|Get(acopy) (Variables|Default|GetLevelNameList) _result_2))
                (bind _asbp_game_instance_3 (Utilities|ConvertGameInstance))
                (Variables|/Game/blueprints/props/BP_GameInstance.BP_GameInstance_C|SetCollected_Cristal_Number _asbp_game_instance_3 0)))))
        (else
          (bind _foundwidgets (Widget|GetAllWidgetsOfClass "/Game/blueprints/props/BP_UI.BP_UI_C" true))
          (Default|PlayFlicerAnimation (Utilities|Array|Get(acopy) _foundwidgets)))))))

(event EventTick
  (params (DeltaSeconds :type Float%20%28single-precision%29)))

(event EventBeginPlay
  (bind _outactors (Actor|GetAllActorsOfClass "/Game/blueprints/props/BP_cristal.BP_cristal_C"))
  (bind _asbp_game_instance (Utilities|ConvertGameInstance))
  (Variables|/Game/blueprints/props/BP_GameInstance.BP_GameInstance_C|SetAllCristalNumber _asbp_game_instance (Utilities|Array|Length _outactors)))

(fn ConstructionScript)

(fn IsLastLevel
  (bind _levelnamelist (Variables|Default|GetLevelNameList))
  (bind _returnvalue (Game|GetCurrentLevelName true))
  (return (== (Utilities|Array|LastIndex _levelnamelist) (Utilities|Array|FindItem _levelnamelist (Utilities|String|StringToName _returnvalue)))))

(fn GetCurrentLevelIndex
  (bind _returnvalue (Game|GetCurrentLevelName true))
  (return (Utilities|Array|FindItem (Variables|Default|GetLevelNameList) (Utilities|String|StringToName _returnvalue))))

(fn SaveLevelTime
  (bind _foundwidgets (Widget|GetAllWidgetsOfClass "/Game/blueprints/props/BP_UI.BP_UI_C" true))
  (bind _asbp_game_instance (Utilities|ConvertGameInstance))
  (Variables|/Game/blueprints/props/BP_GameInstance.BP_GameInstance_C|SetGameTime _asbp_game_instance (Variables|/Game/blueprints/props/BP_UI.BP_UI_C|GetLevelTime (Utilities|Array|Get(acopy) _foundwidgets))))