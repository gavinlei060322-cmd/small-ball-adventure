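; Collectible crystal prop that flies into the player when overlapped and increments the crystal count in the Game Instance.
; On overlap with the player it caches its location, scale and point light intensity, then plays a timeline.
; Timeline alphas lerp it toward the player's live position while shrinking it and fading the light to zero.
; When the timeline finishes, it updates the count and destroys itself.
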(event Collision|EventActorBeginOverlap
  (params (OtherActor :type Actor%20Object%20Reference))
  (Utilities|Isplayer OtherActor
    (:true
      (|CollapseGraph)
      (bind (_direction _location_alpha _scale_alpha _newtrack_2) (Timeline|Timeline Play)
        (:Update
          (CallFunction|GetLocation _location_alpha)
          (CallFunction|ScaleAnimation _scale_alpha)
          (CallFunction|IntensityAnimation _newtrack_2))
        (:Finished
          (bind _asbp_game_instance (Utilities|ConvertGameInstance))
          (Default|IncreaseNumberCrystal _asbp_game_instance)
          (Actor|DestroyActor))))))

(fn ConstructionScript)

(fn GetLocation
  (params (Alpha :type Float%20%28single-precision%29))
  (Transformation|SetActorLocation (Math|Vector|Lerp(Vector) (Variables|Default|GetstartLocation) (Transformation|GetActorLocation (Game|Player|GetPlayerPawn 0)) Alpha) false false))

(fn ScaleAnimation
  (params (Alpha :type Float%20%28single-precision%29))
  (Transformation|SetActorScale3D (Math|Vector|Lerp(Vector) (Variables|Default|Getscale) "0, 0, 0" Alpha)))

(fn IntensityAnimation
  (params (Alpha :type Float%20%28double-precision%29))
  (Rendering|Components|Light|SetIntensity (Variables|Default|GetPointLight) (Math|Float|Lerp (Variables|Default|Getintensity) 0.0 Alpha)))